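; Base pickup actor that adds its type to the player's inventory when BP_Player overlaps it.
; The inventory lives on the BP_WanderingSpirits_GI game instance, and the pickup destroys itself once added.
; The construction script applies the configured static mesh and material, so each pickup's look is driven by variables.
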(event EventBeginPlay)

(event Collision|EventActorBeginOverlap
  (params (OtherActor :type Actor%20Object%20Reference))
  (Utilities|Casting|CastToBP_Player OtherActor)
  (bind _asbp_wandering_spirits_gi (Utilities|Casting|CastToBP_WanderingSpirits_GI (Game|GetGameInstance)))
  (Utilities|Array|Add (Variables|/Game/Blueprints/BP_WanderingSpirits_GI.BP_WanderingSpirits_GI_C|GetInventory _asbp_wandering_spirits_gi) (Variables|Default|GetType))
  (Actor|DestroyActor))

(event EventTick
  (params (DeltaSeconds :type Float%20%28single-precision%29)))

(fn ConstructionScript
  (Components|StaticMesh|SetStaticMesh (Variables|Components|GetMesh) (Variables|Default|GetPickUpMesh))
  (Rendering|Material|SetMaterial (Variables|Components|GetMesh) 0 (Variables|Default|GetMaterial)))