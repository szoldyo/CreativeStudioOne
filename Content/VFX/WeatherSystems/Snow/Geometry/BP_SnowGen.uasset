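; Generated dynamic mesh actor that builds a snow layer over a chosen list of mesh actors using Geometry Script.
; On rebuild, it merges those meshes in world space, raycasts down at seeded random points, and appends small spheres at hits.
; After conversion to local space, an optional remesh thickens and smooths the spheres, then adds box UVs, tangents and normals.
; Tick only prints the game instance's Snowing state.
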(event EventTick
  (params (DeltaSeconds :type Float%20%28single-precision%29))
  (bind _asbp_game_instance (Utilities|Casting|CastToBP_GameInstance (Game|GetGameInstance)))
  (if (Variables|/Game/ThirdPerson/Blueprints/BP_GameInstance.BP_GameInstance_C|Getsnowing _asbp_game_instance)
    (Development|PrintText "Snowing")
    (else
      (Development|PrintText "Not Snowing"))))

(event Events|EventOnRebuildGeneratedMesh
  (params (TargetMesh :type Dynamic%20Mesh%20Object%20Reference))
  (Variables|Default|SetTarget%20Mesh TargetMesh)
  (Utilities|FlowControl|Sequence
    (:then_0
      ;[0 0 0 0.502] Variable: Allows meshes to be added to the BP (snow is applied to these meshes)
      (bind _returnvalue (DynamicMeshActor|AllocateComputeMesh))
      (Variables|Default|SetRaycast%20Mesh%20Actors _returnvalue)
      (for _array_element (Variables|Default|GetMeshesToAddSnowTo)
        (bind _returnvalue_2 (DynamicMeshActor|AllocateComputeMesh))
        (bind _returnvalue_3 (GeometryScript|Scene|CopyMeshfromComponent :Component (Variables|/Script/Engine.Actor|GetRootComponent _array_element) :ToDynamicMesh _returnvalue_2 :bTransformToWorld true :Debug 0)
          (:Failure
            _)
          (:Success
            (GeometryScript|MeshEdits|AppendMesh :TargetMesh (Variables|Default|GetRaycast%20Mesh%20Actors) :AppendMesh _returnvalue_3 :AppendOptions "(CombineMode=EnableAllMatching)" :Debug 0)))
        (Class|DynamicMeshActor|ReleaseComputeMesh _returnvalue_2)))
    (:then_1
      ;[0 0 0 0.502] BVH that raycasts spheres over the meshes (snow is created using the spheres)
      (bind (_outputbvh _returnvalue_4) (Class|GeometryScriptLibraryMeshSpatial|BuildBVHforMesh (Variables|Default|GetRaycast%20Mesh%20Actors) 0))
      (Variables|Default|SetOutput%20BVH _outputbvh)
      (for _index (range 0 (Variables|Default|GetNumberOfSpheres))
        (bind _hitresult (Class|GeometryScriptLibraryMeshSpatial|FindNearestRayIntersectionwithMesh :TargetMesh (Variables|Default|GetRaycast%20Mesh%20Actors) :QueryBVH (Variables|Default|GetOutput%20BVH) :RayOrigin (Math|Vector|MakeVector (Math|Random|RandomFloatinRangefromStream (Variables|Default|GetStream) (.x (.min (Class|GeometryScriptLibraryMeshQueryFunctions|GetMeshBoundingBox _returnvalue_4))) (.x (.max (Class|GeometryScriptLibraryMeshQueryFunctions|GetMeshBoundingBox _returnvalue_4)))) (Math|Random|RandomFloatinRangefromStream (Variables|Default|GetStream) (.y (.min (Class|GeometryScriptLibraryMeshQueryFunctions|GetMeshBoundingBox _returnvalue_4))) (.y (.max (Class|GeometryScriptLibraryMeshQueryFunctions|GetMeshBoundingBox _returnvalue_4)))) (+ (- (.z (.min (Class|GeometryScriptLibraryMeshQueryFunctions|GetMeshBoundingBox _returnvalue_4))) (.z (.max (Class|GeometryScriptLibraryMeshQueryFunctions|GetMeshBoundingBox _returnvalue_4)))) 1e+04)) :RayDirection "0.000000,0.000000,-1.000000" :Debug 0)
          (:Found
            (Class|GeometryScriptLibraryMeshPrimitiveFunctions|AppendSphereBox :TargetMesh (Variables|Default|GetTarget%20Mesh) :Transform (Math|Transform|MakeTransform (.hitposition _hitresult) "0, 0, 0" "1.000000,1.000000,1.000000") :Radius 2.5 :Debug 0)))))
    (:then_2
      ;[0 0 0 0.502] Positions generated snow over the original mesh
      (GeometryScript|Transforms|TransformMesh (Variables|Default|GetTarget%20Mesh) (Math|Transform|InvertTransform (Transformation|GetActorTransform)) true 0))
    (:then_3
      ;[0 0 0 0.502] Creates voxelised mesh over the previously generated spheres (smoothed to improve UVs), normals and tangents are generated
      (if (Variables|Default|GetRemesh)
        (bind _returnvalue_5 (Class|GeometryScriptLibraryMeshVoxelFunctions|ApplyMeshMorphology (Variables|Default|GetTarget%20Mesh) (Utilities|Struct|MakeGeometryScriptMorphologyOptions "(SizeMethod=GridResolution,GridCellSize=0.500000,GridResolution=64)" false (Utilities|Struct|MakeGeometryScript3DGridParameters "GridResolution" 0.5 64) "Dilate" (Variables|Default|GetSnowThickness)) 0))
        (bind _returnvalue_6 (Class|GeometryScriptLibraryMeshDeformFunctions|ApplyIterativeSmoothingtoMesh :TargetMesh _returnvalue_5 :Options (Utilities|Struct|MakeGeometryScriptIterativeMeshSmoothingOptions (Variables|Default|GetSmoothIterations) 0.2 "FullMeshSelection") :Debug 0))
        (bind _returnvalue_7 (Class|GeometryScriptLibraryMeshUVFunctions|SetMeshUVsfromBoxProjection :TargetMesh _returnvalue_6 :BoxTransform (Math|Transform|MakeTransform "0, 0, 0" "0, 0, 0" (- (.max (Class|GeometryScriptLibraryMeshQueryFunctions|GetMeshBoundingBox _returnvalue_6)) (.min (Class|GeometryScriptLibraryMeshQueryFunctions|GetMeshBoundingBox _returnvalue_6)))) :Debug 0))
        (bind _returnvalue_8 (Class|GeometryScriptLibraryMeshNormalsFunctions|ComputeTangents :TargetMesh _returnvalue_7 :Debug 0))
        (Class|GeometryScriptLibraryMeshNormalsFunctions|ComputeSplitNormals :TargetMesh _returnvalue_8 :SplitOptions (Utilities|Struct|MakeGeometryScriptSplitNormalsOptions true 8e+01 false "(bDefaultLayer=True,ExtendedLayerIndex=0)") :Debug 0)))
    (:then_4
      (DynamicMeshActor|ReleaseAllComputeMeshes))))

(fn ConstructionScript)